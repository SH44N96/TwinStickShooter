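; Twin-stick enemy character that damages the hero on contact and awards score to the game mode when killed.
; Overlapping the hero starts a looping timer that deals damage at the attack rate, cleared when the overlap ends.
; On death it detaches its controller, removes the damage volume and loosens collision, then explodes and destroys itself after a delay.
; The construction script tints the body through a dynamic material instance.
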(event `self.ReceiveActorEndOverlap`
  (params (OtherActor :type "Actor Object Reference"))
  (if (== OtherActor (`self.Hero`))
    (`KismetSystemLibrary.K2_ClearTimer` null "DamageTheHero")))

(event `self.ReceiveActorBeginOverlap`
  (params (OtherActor :type "Actor Object Reference"))
  (`parent.ReceiveActorBeginOverlap` OtherActor)
  (bind _ashero_character (cast `/Game/Blueprints/HeroCharacter` OtherActor))
  (set `self.Hero` _ashero_character)
  (`KismetSystemLibrary.K2_SetTimer` null "DamageTheHero" (/ 1.0 (`self.AttacksPerSecond`)) true))

(event `AffectHealth`
  (params (Delta :type "Float (double-precision)"))
  (bind _capsulecomponent (`self.CapsuleComponent`))
  (`self.CalculateHealth` Delta)
  (if (`self.IsDead`)
    (bind _astwin_stick_mode (cast `/Game/Blueprints/TwinStickMode` (`GameplayStatics.GetGameMode`)))
    (`/Game/Blueprints/TwinStickMode.IncrementScore` _astwin_stick_mode (`self.Score`))
    (`self.DetachFromControllerPendingDestroy`)
    (`ActorComponent.K2_DestroyComponent` (`self.DamageVolume`))
    (`PrimitiveComponent.SetCollisionResponseToChannel` _capsulecomponent "ECC_WorldDynamic" "ECR_Ignore")
    (`PrimitiveComponent.SetCollisionResponseToChannel` _capsulecomponent "ECC_Pawn" "ECR_Ignore")
    (`KismetSystemLibrary.Delay` 3.0)
    (`|SpawnActorFromClass` "/Game/Blueprints/Explosion.Explosion_C" (`self.GetTransform`) "Undefined" "OverrideRootScale" null null)
    (`self.K2_DestroyActor`)))

(event `DamageTheHero`
  (`/Game/Blueprints/HeroCharacter.AffectHealth` (`self.Hero`) (`self.Damage`)))

(fn `UserConstructionScript`
  (`parent.UserConstructionScript`)
  (bind _returnvalue (`PrimitiveComponent.CreateDynamicMaterialInstance` (`self.Mesh`) 0 null "None"))
  (bind _output_get (set `self.DynaMat` _returnvalue))
  (`MaterialInstanceDynamic.SetVectorParameterValue` _output_get "BodyColor" (`self.EnemyColor`)))