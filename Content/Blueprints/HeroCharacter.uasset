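; HeroCharacter is the player character for a twin-stick shooter, with movement, mouse aiming, firing, health and score.
; On BeginPlay it attaches a spawned weapon to GunSocket, records its spawn transform in TwinStickMode and creates the HUD.
; While MouseHover is set, Tick turns control rotation toward the cursor's offset from screen center.
; Death disables input, then after a delay requests a GameMode respawn and destroys weapon and hero.
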(event `self.ReceiveBeginPlay`
  (bind _mesh (`self.Mesh`))
  (`parent.ReceiveBeginPlay`)
  (`|ExecutionSequence`
    (:`then_0`
      (bind _returnvalue (`|SpawnActorFromClass` "/Game/Blueprints/Weapon.Weapon_C" (`SceneComponent.K2_GetComponentToWorld` _mesh) "Undefined" "OverrideRootScale" null null))
      (bind _output_get (set `self.Weapon` _returnvalue))
      (`self.K2_AttachToComponent` _output_get _mesh "GunSocket" "SnapToTarget" "SnapToTarget" "KeepRelative" true))
    (:`then_1`
      (bind _astwin_stick_mode (cast `/Game/Blueprints/TwinStickMode` (`GameplayStatics.GetGameMode`)))
      (bind _output_get_2 (set `self.GameMode` _astwin_stick_mode))
      (set `/Game/Blueprints/TwinStickMode.PlayerSpawnTransform` (`self.GetTransform`) _output_get_2))
    (:`then_2`
      (bind _returnvalue_2 (`|CreateWidget` "/Game/Blueprints/TwinStickHUD.TwinStickHUD_C"))
      (`UserWidget.AddToViewport` _returnvalue_2 0))))

(event `InputAxis|MoveUp`
  (params (AxisValue :type "Float (single-precision)"))
  ;[1 1 1] Movement
  (`self.AddMovementInput` (1.0 0.0 0.0) AxisValue))

(event `self.ReceiveTick`
  (params (DeltaSeconds :type "Float (single-precision)"))
  (bind (_locationx _locationy) (`WidgetLayoutLibrary.GetMousePositionScaledByDPI` (`GameplayStatics.GetPlayerController` 0)))
  (bind (_returnvalue_x _returnvalue_y) (`KismetMathLibrary.BreakVector2D` (/ (/ (`WidgetLayoutLibrary.GetViewportSize`) (`WidgetLayoutLibrary.GetViewportScale`)) 2.0)))
  ;[1 1 1] Rotation
  (if (`self.MouseHover`)
    (`Controller.SetControlRotation` (`GameplayStatics.GetPlayerController` 0) (`KismetMathLibrary.Conv_VectorToRotator` (`KismetMathLibrary.MakeVector` (* (- _locationy _returnvalue_y) -1.0) (- _locationx _returnvalue_x))))))

(event `InputAction|MouseFire`
  (params (Key :type "Key Structure"))
  (bind _weapon (`self.Weapon`))
  (:`Pressed`
    (`/Game/Blueprints/Weapon.PullTrigger` _weapon))
  (:`Released`
    (`/Game/Blueprints/Weapon.ReleaseTrigger` _weapon)))

(event `InputAxis|MoveRight`
  (params (AxisValue :type "Float (single-precision)"))
  ;[1 1 1] Movement
  (`self.AddMovementInput` (0.0 1.0 0.0) AxisValue))

(event `AffectHealth`
  (params (Delta :type "Float (double-precision)"))
  (`self.CalculateHealth` Delta)
  (if (`self.IsDead`)
    (set `self.MouseHover` false)
    (`self.DisableInput` null)
    (`KismetSystemLibrary.Delay` 3.0)
    (`/Game/Blueprints/TwinStickMode.RespawnPlayer` (`self.GameMode`))
    (`self.K2_DestroyActor` (`self.Weapon`))
    (`self.K2_DestroyActor` self)))

(event `IncrementScore`
  (params (DeltaScore :type Integer))
  (set `self.Score` (+ DeltaScore (`self.Score`))))

(fn `UserConstructionScript`
  (`parent.UserConstructionScript`)
  (bind _returnvalue (`PrimitiveComponent.CreateDynamicMaterialInstance` (`self.Mesh`) 0 null "None"))
  (bind _output_get (set `self.DynaMat` _returnvalue))
  (`MaterialInstanceDynamic.SetVectorParameterValue` _output_get "BodyColor" (`self.HeroColor`)))